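; Skeleton melee enemy that damages the VR player or debugging pawn and dies with a sound.
; An attack flag gates overlap damage from a hitbox, whose collision is toggled by functions named for animation notifies.
; Health component events spawn floating damage-number widget actors and destroy the skeleton on death.
; It also exposes animation pause and state-reset hooks; the hit-reaction flag is never set, and patrol points only drive debug prints.
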(event `self.ReceiveBeginPlay`
  (`PrimitiveComponent.SetCollisionEnabled` (`self.AttackHitbox`) "NoCollision")
  (bind _asenemy_controller (cast `EnemyController` (`self.GetController`))
    (:`then`
      (for _ (`EnemyController.InternalPatrolPoints` _asenemy_controller)
        (`KismetSystemLibrary.PrintString` "Hello")))
    (:`CastFailed`
      (`KismetSystemLibrary.PrintString` "no control"))))

(event `self.ExecuteAttack1`
  ;[1 1 1] Attack damage handling
  (set `self.IsAttacking` true))

(event `self.AttackHitbox.OnComponentBeginOverlap`
  (params (OverlappedComponent :type "PrimitiveComponent Object Reference") (OtherActor :type "Actor Object Reference") (OtherComp :type "PrimitiveComponent Object Reference") (OtherBodyIndex :type Integer) (bFromSweep :type Boolean) (SweepResult :type "HitResult Structure (by ref)"))
  ;[1 1 1] Attack damage handling
  (if (`self.IsAttacking`)
    (bind _asvrpawn (cast `/Game/blueprints/PlayerTypes/VRPawn` OtherActor)
      (:`then`
        (`VRCharacterComponent.TakeDamage` (`/Game/blueprints/PlayerTypes/VRPawn.VRCharacterComp` _asvrpawn) (`self.MeleeAttack1Damage`)))
      (:`CastFailed`
        (bind _asdebugging_pawn_bp (cast `/Game/blueprints/PlayerTypes/DebuggingPawnBP` OtherActor))
        (`EnemyBaseComponent.TakeDamage` (`/Game/blueprints/PlayerTypes/DebuggingPawnBP.EnemyBaseComp` _asdebugging_pawn_bp) (`self.MeleeAttack1Damage`))))))

(event `self.HealthComponent.OnDamaged`
  (params (DamageTaken :type "Float (single-precision)"))
  ;[1 1 1] Connect OnDamaged to setting HasTakenDamage to true when an animation blueprint is implemented
  (`self.SpawnDamageUI` DamageTaken))

(event `self.FreezeAnimations`
  (set `SkeletalMeshComponent.bPauseAnims` true (`self.Mesh`)))

(event `self.UnfreezeAnimations`
  (set `SkeletalMeshComponent.bPauseAnims` false (`self.Mesh`)))

(event `self.HealthComponent.OnDeath`
  (`self.K2_DestroyActor`)
  (`GameplayStatics.PlaySoundAtLocation` "/Game/Models/Sounds/SkeletonDeathSFX.SkeletonDeathSFX" (`self.K2_GetActorLocation`) (struct) 1.0 1.0 0.0 null null null null))

(fn `DespawnHitboxOnAnimEnd`
  (`PrimitiveComponent.SetCollisionEnabled` (`self.AttackHitbox`) "NoCollision"))

(fn `GetMesh`
  (returns (NewParam :type "SkeletalMeshComponent Object Reference"))
  (return (`self.Mesh`)))

(fn `ResetHasTakenDamage`
  (set `self.HasTakenDamage` false))

(fn `SpawnDamageUI`
  (params (InDamage :type "Float (double-precision)"))
  (locals (DamageTaken :type "Float (double-precision)") (InstancedActor :type "/Game/blueprints/UI/UIActors/DamageWidgetActor Object Reference"))
  (set `local.DamageTaken` InDamage)
  (bind _returnvalue (`|SpawnActorFromClass` "/Game/blueprints/UI/UIActors/DamageWidgetActor.DamageWidgetActor_C" (`SceneComponent.K2_GetComponentToWorld` (`self.UISpawnPoint`)) "Undefined" "OverrideRootScale" null null))
  (bind _output_get (set `local.InstancedActor` _returnvalue))
  (bind _asdamage_widget (cast `/Game/blueprints/UI/WidgetBlueprints/DamageWidget` (`WidgetComponent.GetWidget` (`/Game/blueprints/UI/UIActors/DamageWidgetActor.Damage` _output_get))))
  (`/Game/blueprints/UI/WidgetBlueprints/DamageWidget.AddAndLift` _asdamage_widget (`KismetMathLibrary.FTrunc` (`local.DamageTaken`)))
  (set `/Game/blueprints/UI/UIActors/DamageWidgetActor.ShouldAdjust` true (`local.InstancedActor`)))

(fn `SpawnHitboxOnAnimNotify`
  (`PrimitiveComponent.SetCollisionEnabled` (`self.AttackHitbox`) "QueryAndPhysics")
  (`KismetSystemLibrary.PrintString` "Hello"))

(fn `SwitchAnimStates`
  (set `self.IsAttacking` false))

(fn `UserConstructionScript`
  (`ActorComponent.SetAutoActivate` (`self.AttackHitbox`) false))