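; SlimeEnemy is an enemy Blueprint that deals contact damage to the VR player.
; Hitbox hits on a player-tagged VRPawn apply damage through its VRCharacterComp.
; HealthComponent events set the death flag and spawn a lifting damage-number widget actor at UISpawnPoint.
; Ground events set a jump flag (Saltar), and freeze/unfreeze events toggle Hitbox physics, though both pause mesh animations.
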(event `self.ReceiveBeginPlay`)

(event `self.ReceiveTick`
  (params (DeltaSeconds :type "Float (single-precision)")))

(event `self.OnGroundEvent2`
  (set `self.Saltar` true))

(event `self.FreezeAnimations`
  (set `SkeletalMeshComponent.bPauseAnims` true (`self.CharacterMesh`))
  (`PrimitiveComponent.SetSimulatePhysics` (`self.Hitbox`) false))

(event `self.UnfreezeAnimations`
  (set `SkeletalMeshComponent.bPauseAnims` true (`self.CharacterMesh`))
  (`PrimitiveComponent.SetSimulatePhysics` (`self.Hitbox`) true))

(event `self.HealthComponent.OnDeath`
  (set `self.HasDied` true))

(event `self.HealthComponent.OnDamaged`
  (params (DamageTaken :type "Float (single-precision)"))
  (`self.SpawnDamageUI` DamageTaken))

(event `self.Hitbox.OnComponentHit`
  (params (HitComponent :type "PrimitiveComponent Object Reference") (OtherActor :type "Actor Object Reference") (OtherComp :type "PrimitiveComponent Object Reference") (NormalImpulse :type "Vector Structure") (Hit :type "HitResult Structure (by ref)"))
  (if (`self.ActorHasTag` OtherActor "PlayerTag")
    (bind _asvrpawn (cast `/Game/VRTemplate/Blueprints/VRPawn` OtherActor))
    (`VRCharacterComponent.TakeDamage` (`/Game/VRTemplate/Blueprints/VRPawn.VRCharacterComp` _asvrpawn) (`self.Damage`))))

(fn `SpawnDamageUI`
  (params (InDamage :type "Float (double-precision)"))
  (locals (InstancedActor :type "/Game/blueprints/UI/WidgetBlueprints/DamageWidgetActor Object Reference"))
  (bind _returnvalue (`|SpawnActorFromClass` "/Game/blueprints/UI/WidgetBlueprints/DamageWidgetActor.DamageWidgetActor_C" (`SceneComponent.K2_GetComponentToWorld` (`self.UISpawnPoint`)) "Undefined" "OverrideRootScale" null null))
  (bind _output_get (set `local.InstancedActor` _returnvalue))
  (bind _asdamage_widget (cast `/Game/blueprints/UI/WidgetBlueprints/DamageWidget` (`WidgetComponent.GetWidget` (`/Game/blueprints/UI/WidgetBlueprints/DamageWidgetActor.Damage` _output_get))))
  (`/Game/blueprints/UI/WidgetBlueprints/DamageWidget.AddAndLift` _asdamage_widget (`KismetMathLibrary.FTrunc` InDamage))
  (set `/Game/blueprints/UI/WidgetBlueprints/DamageWidgetActor.ShouldAdjust` true (`local.InstancedActor`)))

(fn `UserConstructionScript`)