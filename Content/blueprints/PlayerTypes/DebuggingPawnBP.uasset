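; Debug player pawn that casts elemental magic: fireball, lightning or a time freeze on enemies.
; Switch input cycles the element array and updates the element icon; attack dispatches to the matching spell component.
; On BeginPlay it attaches the level's UIActor to itself and updates its widgets directly through casts.
; It reuses EnemyBaseComp for player health, refreshing the health bar on damage; the death handler is empty.
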(event `self.AttackOne`
  (`self.HandleAttack`))

(event `self.SwitchElement`
  (`self.HandleElementSwitch`))

(event `self.ReceiveBeginPlay`
  (bind _returnvalue (`GameplayStatics.GetActorOfClass` "/Game/blueprints/UI/UIActors/UIActor.UIActor_C"))
  (`self.K2_AttachToComponent` _returnvalue (`self.DummyGUIAttachPoint`) "None" "KeepRelative" "KeepRelative" "KeepRelative" false)
  (set `self.PassedUIRef` _returnvalue))

(event `self.EnemyBaseComp.OnDeath`
  (`self.FallecioFunc`))

(event `self.EnemyBaseComp.OnDamaged`
  (params (DamageTaken :type "Float (single-precision)"))
  (`self.UpdateHealthGUI`))

(fn `FallecioFunc`)

(fn `HandleAttack`
  (if (`KismetStringLibrary.EqualEqual_StrStr` (`self.SelectedElement`) "Fire")
    (`FireballComponent.Fire` (`self.FireballSpawner`) 20.0 1000.0 40.0 "/Game/Models/Fireball/FireballSphere.FireballSphere" "/Game/Models/Fireball/ico.ico" (`self.K2_GetActorLocation`) (`self.GetActorForwardVector`) (`self.K2_GetActorRotation`) null)
    (elif (`KismetStringLibrary.EqualEqual_StrStr` (`self.SelectedElement`) "Lightning")
      (`LightningAttackComponent.FireLightning` (`self.LightningSpawner`) null (`self.K2_GetActorLocation`) (`self.GetActorForwardVector`) (`self.K2_GetActorRotation`) self)
      (elif (`KismetStringLibrary.EqualEqual_StrStr` (`self.SelectedElement`) "Time")
        (`TimeMagicComponent.FreezeEnemies` (`self.TimeMagic`))))))

(fn `HandleElementSwitch`
  (bind _output_get (set `self.CurrentElementIndex` (+ (`self.CurrentElementIndex`) 1)))
  (if (> _output_get (- (`KismetArrayLibrary.Array_Length` (`self.ElementArray`)) 1))
    (set `self.CurrentElementIndex` 0)
    (set `self.SelectedElement` (`|GetArrayItem` (`self.ElementArray`) (`self.CurrentElementIndex`)))
    (`self.PassElementImage`)
    (else
      (set `self.SelectedElement` (`|GetArrayItem` (`self.ElementArray`) (`self.CurrentElementIndex`)))
      (`self.PassElementImage`))))

(fn `PassElementImage`
  (if (`KismetStringLibrary.EqualEqual_StrStr` (`self.SelectedElement`) "Fire")
    (bind _aselement_widget (cast `/Game/blueprints/UI/WidgetBlueprints/ElementWidget` (`WidgetComponent.GetWidget` (`/Game/blueprints/UI/UIActors/UIActor.Element` (`self.PassedUIRef`))))
      (:`then`
        (`Image.SetBrush` (`/Game/blueprints/UI/WidgetBlueprints/ElementWidget.Image_68` _aselement_widget) (make `SlateBrush` (32.0 32.0) (struct) (struct :`SpecifiedColor` (struct :`R` 1.0 :`G` 1.0 :`B` 1.0 :`A` 1.0) :`ColorUseRule` "UseColor_Specified") (struct :`CornerRadii` (struct :`W` 1.0) :`Color` (struct :`SpecifiedColor` (struct) :`ColorUseRule` "UseColor_Specified") :`RoundingType` "HalfHeightRadius") "/Game/blueprints/UI/Images/FirePNG.FirePNG")))
      (:`CastFailed`
        (`KismetSystemLibrary.PrintString` ":(")))
    (elif (`KismetStringLibrary.EqualEqual_StrStr` (`self.SelectedElement`) "Lightning")
      (bind _aselement_widget_2 (cast `/Game/blueprints/UI/WidgetBlueprints/ElementWidget` (`WidgetComponent.GetWidget` (`/Game/blueprints/UI/UIActors/UIActor.Element` (`self.PassedUIRef`))))
        (:`then`
          (`Image.SetBrush` (`/Game/blueprints/UI/WidgetBlueprints/ElementWidget.Image_68` _aselement_widget_2) (make `SlateBrush` (32.0 32.0) (struct) (struct :`SpecifiedColor` (struct :`R` 1.0 :`G` 1.0 :`B` 1.0 :`A` 1.0) :`ColorUseRule` "UseColor_Specified") (struct :`CornerRadii` (struct :`W` 1.0) :`Color` (struct :`SpecifiedColor` (struct) :`ColorUseRule` "UseColor_Specified") :`RoundingType` "HalfHeightRadius") "/Game/blueprints/UI/Images/LightningPNG.LightningPNG")))
        (:`CastFailed`
          (`KismetSystemLibrary.PrintString` ":(2")))
      (elif (`KismetStringLibrary.EqualEqual_StrStr` (`self.SelectedElement`) "Time")
        (bind _aselement_widget_3 (cast `/Game/blueprints/UI/WidgetBlueprints/ElementWidget` (`WidgetComponent.GetWidget` (`/Game/blueprints/UI/UIActors/UIActor.Element` (`self.PassedUIRef`)))))
        (`Image.SetBrush` (`/Game/blueprints/UI/WidgetBlueprints/ElementWidget.Image_68` _aselement_widget_3) (make `SlateBrush` (32.0 32.0) (struct) (struct :`SpecifiedColor` (struct :`R` 1.0 :`G` 1.0 :`B` 1.0 :`A` 1.0) :`ColorUseRule` "UseColor_Specified") (struct :`CornerRadii` (struct :`W` 1.0) :`Color` (struct :`SpecifiedColor` (struct) :`ColorUseRule` "UseColor_Specified") :`RoundingType` "HalfHeightRadius") "/Game/blueprints/UI/Images/TimePNG.TimePNG"))))))

(fn `UpdateHealthGUI`
  (bind _enemybasecomp (`self.EnemyBaseComp`))
  (bind _ashealth_widget (cast `/Game/blueprints/UI/WidgetBlueprints/HealthWidget` (`WidgetComponent.GetWidget` (`/Game/blueprints/UI/UIActors/UIActor.Health` (`self.PassedUIRef`)))))
  (`ProgressBar.SetPercent` (`/Game/blueprints/UI/WidgetBlueprints/HealthWidget.Healthbar` _ashealth_widget) (/ (/ (* (`EnemyBaseComponent.GetHealth` _enemybasecomp) 100.0) (`EnemyBaseComponent.GetMaxHealth` _enemybasecomp)) 100.0)))

(fn `UserConstructionScript`)