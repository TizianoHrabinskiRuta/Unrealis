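; VR player character with hand grabbing, stick locomotion and health.
; Each grab input sends GrabMessage with its motion controller to every Grippableinterface actor in that hand's sphere, but stores only the last for release.
; Left-axis input moves the character along the camera's forward and right vectors at reduced scale.
; TakeDamageWrapper forwards damage to HealthBase, whose death event only prints a message.
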(event `InputAction|GrabLeft`
  (params (Key :type "Key Structure"))
  (bind _grableftactors (`self.GrabLeftActors`))
  (:`Pressed`
    (for _array_element (`PrimitiveComponent.GetOverlappingActors` (`self.SphereLeft`) null)
      (if (`KismetSystemLibrary.DoesImplementInterface` _array_element "/Game/interface/grippableinterface.grippableinterface_C")
        (message `/Game/interface/grippableinterface.Grab` _array_element (`self.MotionControllerLeft`))
        (set `self.GrabLeftActors` _array_element))))
  (:`Released`
    (`/Engine/EditorBlueprintResources/StandardMacros.IsValid` _grableftactors
      (:`Is Valid`
        (message `/Game/interface/grippableinterface.Release` _grableftactors)))))

(event `InputAction|GrabRight`
  (params (Key :type "Key Structure"))
  (bind _grabrightactors (`self.GrabRightActors`))
  (:`Pressed`
    (for _array_element (`PrimitiveComponent.GetOverlappingActors` (`self.SphereRight`) null)
      (if (`KismetSystemLibrary.DoesImplementInterface` _array_element "/Game/interface/grippableinterface.grippableinterface_C")
        (message `/Game/interface/grippableinterface.Grab` _array_element (`self.MotionControllerRight`))
        (set `self.GrabRightActors` _array_element))))
  (:`Released`
    (`/Engine/EditorBlueprintResources/StandardMacros.IsValid` _grabrightactors
      (:`Is Valid`
        (message `/Game/interface/grippableinterface.Release` _grabrightactors)))))

(event `InputAxis|MovementAxisLeft_X`
  (params (AxisValue :type "Float (single-precision)"))
  (`self.AddMovementInput` (`SceneComponent.GetRightVector` (`self.Camera`)) (/ AxisValue 1.5)))

(event `InputAxis|MovementAxisLeft_Y`
  (params (AxisValue :type "Float (single-precision)"))
  (`self.AddMovementInput` (`SceneComponent.GetForwardVector` (`self.Camera`)) (/ AxisValue 1.5)))

(event `self.HealthBase.OnDeath`
  (`KismetSystemLibrary.PrintString` "Player Has died"))

(fn `Take Damage Wrapper`
  (params (Damage :type "Float (double-precision)"))
  (`EnemyBaseComponent.TakeDamage` (`self.HealthBase`) Damage))

(fn `UserConstructionScript`)