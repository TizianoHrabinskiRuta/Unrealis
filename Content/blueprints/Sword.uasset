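; Sword actor that can be grabbed and released by a motion controller and deals damage to actors it touches.
; Grab stores the passed component and attaches to it, keeping the world transform.
; Release detaches the static mesh if that component is valid and turns on physics simulation.
; Any overlap on the mesh applies a fixed amount of damage, with no filtering or swing-speed check.
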(event `self.StaticMesh.OnComponentBeginOverlap`
  (params (OverlappedComponent :type "PrimitiveComponent Object Reference") (OtherActor :type "Actor Object Reference") (OtherComp :type "PrimitiveComponent Object Reference") (OtherBodyIndex :type Integer) (bFromSweep :type Boolean) (SweepResult :type "HitResult Structure (by ref)"))
  (`GameplayStatics.ApplyDamage` OtherActor 1.0))

(event `/Game/interface/grippableinterface.Grab`
  (params (Component :type "MotionControllerComponent Object Reference"))
  (set `self.MotionController` Component)
  (`self.K2_AttachToComponent` Component "None" "KeepWorld" "KeepWorld" "KeepWorld"))

(event `/Game/interface/grippableinterface.Release`
  (`/Engine/EditorBlueprintResources/StandardMacros.IsValid` (`self.MotionController`)
    (:`Is Valid`
      (`SceneComponent.K2_DetachFromComponent` (`self.StaticMesh`) "KeepWorld" "KeepWorld" "KeepWorld" true)
      (`PrimitiveComponent.SetSimulatePhysics` (`self.StaticMesh`) true))))

(fn `UserConstructionScript`)