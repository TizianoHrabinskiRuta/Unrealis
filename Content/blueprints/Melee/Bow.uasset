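; Bow weapon with a grabbable draw string, built from two cables whose ends attach to a movable Scene component.
; Construction and Tick attach both cables to that component, and Tick also caps its local Y travel, snapping it back to rest near the lower end.
; Releasing the grab sets Strength from the pull position, though the first comparison makes the two lower tiers unreachable.
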(event `self.ReceiveTick`
  (params (DeltaSeconds :type "Float (single-precision)"))
  (bind (_relativelocation_x _relativelocation_y) (`KismetMathLibrary.BreakVector` (`SceneComponent.RelativeLocation` (`self.Scene`))))
  (bind (_relativelocation_x_2 _relativelocation_y_2) (`KismetMathLibrary.BreakVector` (`SceneComponent.RelativeLocation` (`self.Scene`))))
  (`CableComponent.SetAttachEndToComponent` (`self.CableArriba`) (`self.Scene`) "None")
  (`CableComponent.SetAttachEndToComponent` (`self.CableAbajo`) (`self.Scene`) "None")
  (if (> _relativelocation_y 349.999976)
    (`SceneComponent.K2_SetRelativeLocation` (`self.Scene`) (0.0 349.999976 0.0) false false)
    (elif (< _relativelocation_y_2 169.999989)
      (`SceneComponent.K2_SetRelativeLocation` (`self.Scene`) (0.0 149.999989 0.0) false false))))

(event `self.GrabComponent1.OnDropped`
  (bind (_relativelocation_x _relativelocation_y) (`KismetMathLibrary.BreakVector` (`SceneComponent.RelativeLocation` (`self.Scene`))))
  (bind (_relativelocation_x_2 _relativelocation_y_2) (`KismetMathLibrary.BreakVector` (`SceneComponent.RelativeLocation` (`self.Scene`))))
  (bind (_relativelocation_x_3 _relativelocation_y_3) (`KismetMathLibrary.BreakVector` (`SceneComponent.RelativeLocation` (`self.Scene`))))
  (if (<= _relativelocation_y_2 349.999976)
    (set `self.Strength` 3.0)
    (elif (== _relativelocation_y 299.999979)
      (set `self.Strength` 2.0)
      (elif (== _relativelocation_y_3 249.999982)
        (set `self.Strength` 1.0)))))

(fn `UserConstructionScript`
  (`CableComponent.SetAttachEndToComponent` (`self.CableArriba`) (`self.Scene`) "None")
  (`CableComponent.SetAttachEndToComponent` (`self.CableAbajo`) (`self.Scene`) "None"))