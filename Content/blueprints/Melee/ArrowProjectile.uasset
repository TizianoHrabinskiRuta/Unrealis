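; Arrow projectile actor that deals fixed, heavy damage to enemies its collision sphere overlaps.
; Physics-simulating components get an impulse from the arrow's velocity, then after a brief delay the arrow calls destroy and damages AIEnemyBase or SlimeBase actors.
; Non-simulating hits damage only AIEnemyBase, immediately and without destroying the arrow.
; A stopped arrow destroys itself after a longer delay.
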(event `self.SphereCollision.OnComponentBeginOverlap`
  (params (OverlappedComponent :type "PrimitiveComponent Object Reference") (OtherActor :type "Actor Object Reference") (OtherComp :type "PrimitiveComponent Object Reference") (OtherBodyIndex :type Integer) (bFromSweep :type Boolean) (SweepResult :type "HitResult Structure (by ref)"))
  (if (`SceneComponent.IsSimulatingPhysics` OtherComp "None")
    (`PrimitiveComponent.AddImpulse` OtherComp (* (`MovementComponent.Velocity` (`self.ProjectileMovement`)) 1.0) "None" false)
    (`KismetSystemLibrary.Delay` 0.2)
    (`self.K2_DestroyActor`)
    (bind _asaienemy_base (cast `AIEnemyBase` OtherActor)
      (:`then`
        (`EnemyBaseComponent.TakeDamage` (`AIEnemyBase.GetEnemyBase` _asaienemy_base) 2000.0))
      (:`CastFailed`
        (bind _asslime_base (cast `SlimeBase` OtherActor))
        (`EnemyBaseComponent.TakeDamage` (`SlimeBase.GetEnemyBase` _asslime_base) 2000.0)))
    (else
      (bind _asaienemy_base_2 (cast `AIEnemyBase` OtherActor))
      (`EnemyBaseComponent.TakeDamage` (`AIEnemyBase.GetEnemyBase` _asaienemy_base_2) 2000.0))))

(event `self.ProjectileMovement.OnProjectileStop`
  (params (ImpactResult :type "HitResult Structure (by ref)"))
  (`KismetSystemLibrary.Delay` 10.0)
  (`self.K2_DestroyActor`))

(fn `UserConstructionScript`)