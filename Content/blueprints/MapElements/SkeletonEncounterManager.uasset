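; Map element that tracks the deaths of a group of skeleton enemies in an encounter.
; On BeginPlay it binds a handler to the OnDeath event of each Skeletons entry's EnemyBase.
; OnSkeletonDeath compares KilledSkeletons to the array length, but the counter is never incremented here and the completion branch is empty.
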(event `self.ReceiveBeginPlay`
  (for _array_element (`self.Skeletons`)
    (add `EnemyBaseComponent.OnDeath` (`AIEnemyBase.GetEnemyBase` _array_element) (`|CreateDelegate` :!event `OnSkeletonDeath`))))

(fn `OnSkeletonDeath`
  (if (>= (`self.Killed Skeletons`) (`KismetArrayLibrary.Array_Length` (`self.Skeletons`)))
    _))

(fn `UserConstructionScript`)