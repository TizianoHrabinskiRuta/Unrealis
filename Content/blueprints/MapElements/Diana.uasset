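; Diana is an arrow target map element that reports its first hit to a DianaManager.
; On BeginPlay it scans all DianaManager actors and keeps the one whose ManagerName matches its OwnerName.
; When an ArrowProjectile overlaps its Collision component, it increments that manager's hit counter and sets HasBeenHit, so later arrows are not counted again.
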(event `self.ReceiveBeginPlay`
  (bind _outactors (`GameplayStatics.GetAllActorsOfClass` "/Game/blueprints/MapElements/BaseManagers/DianaManager.DianaManager_C")) ; Gets the registered manager for the target
  (for _array_element _outactors
    (if (`KismetStringLibrary.EqualEqual_StrStr` (`self.OwnerName`) (`/Game/blueprints/MapElements/BaseManagers/DianaManager.ManagerName` _array_element))
      (set `self.OwnerManager` _array_element))))

(event `self.Collision.OnComponentBeginOverlap`
  (params (OverlappedComponent :type "PrimitiveComponent Object Reference") (OtherActor :type "Actor Object Reference") (OtherComp :type "PrimitiveComponent Object Reference") (OtherBodyIndex :type Integer) (bFromSweep :type Boolean) (SweepResult :type "HitResult Structure (by ref)"))
  (cast `/Game/blueprints/Melee/ArrowProjectile` OtherActor)
  (if (not (`self.HasBeenHit`))
    (`/Game/blueprints/MapElements/BaseManagers/DianaManager.IncrementHitCounter` (`self.OwnerManager`))
    (set `self.HasBeenHit` true)))

(fn `UserConstructionScript`)