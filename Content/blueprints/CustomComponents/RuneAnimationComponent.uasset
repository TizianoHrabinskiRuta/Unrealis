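; Actor component that animates its owner, presumably a rune, with a continuous yaw spin and a vertical bob.
; Each Tick adds RotationSpeed to yaw, then steps height up or down, reversing when a tick counter exceeds its limit.
; Motion is per frame without delta time, and the owner is assigned through SetOwner.
; SetMaxHeightChanges writes to the running counters, leaving the limits unchanged.
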(event `self.ReceiveTick`
  (params (DeltaSeconds :type "Float (single-precision)"))
  (bind (_returnvalue_roll _returnvalue_pitch _returnvalue_yaw) (`KismetMathLibrary.BreakRotator` (`Actor.K2_GetActorRotation` (`self.Owner`))))
  (`Actor.K2_SetActorRotation` (`self.Owner`) (`KismetMathLibrary.MakeRotator` _returnvalue_roll _returnvalue_pitch (+ _returnvalue_yaw (`self.RotationSpeed`))) false)
  (`self.HandleElevationChange`))

(fn `HandleElevationChange`
  (bind (_returnvalue_x _returnvalue_y _returnvalue_z) (`KismetMathLibrary.BreakVector` (`Actor.K2_GetActorLocation` (`self.Owner`))))
  (bind (_returnvalue_x_2 _returnvalue_y_2 _returnvalue_z_2) (`KismetMathLibrary.BreakVector` (`Actor.K2_GetActorLocation` (`self.Owner`))))
  (if (`self.IsRising`)
    (`Actor.K2_SetActorLocation` (`self.Owner`) (`KismetMathLibrary.MakeVector` _returnvalue_x_2 _returnvalue_y_2 (+ _returnvalue_z_2 (`self.HeightChangeSpeed`))) false false)
    (bind _output_get (set `self.TotalPositiveHeightChanges` (+ (`self.TotalPositiveHeightChanges`) 1.0)))
    (if (> _output_get (`self.MaxPositiveZChanges`))
      (set `self.IsRising` false)
      (set `self.TotalPositiveHeightChanges` 0.0))
    (else
      (`Actor.K2_SetActorLocation` (`self.Owner`) (`KismetMathLibrary.MakeVector` _returnvalue_x _returnvalue_y (- _returnvalue_z (`self.HeightChangeSpeed`))) false false)
      (bind _output_get_2 (set `self.TotalNegativeHeightChanges` (+ (`self.TotalNegativeHeightChanges`) 1.0)))
      (if (> _output_get_2 (`self.MaxNegativeZChanges`))
        (set `self.IsRising` true)
        (set `self.TotalNegativeHeightChanges` 0.0)))))

(fn `SetHeightChangeSpeed`
  (params (InSpeed :type "Float (double-precision)"))
  (set `self.HeightChangeSpeed` InSpeed))

(fn `SetMaxHeightChanges`
  (params (InMaxNegativeHeightChanges :type "Float (double-precision)") (InMaxPositiveHeightChanges :type "Float (double-precision)"))
  (set `self.TotalPositiveHeightChanges` InMaxPositiveHeightChanges)
  (set `self.TotalNegativeHeightChanges` InMaxNegativeHeightChanges))

(fn `SetOwner`
  (params (NewParam :type "Actor Object Reference"))
  (set `self.Owner` NewParam))