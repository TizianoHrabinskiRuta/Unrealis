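; AnsuzActor is a health pickup that heals the VR player when collected.
; On begin play it plays audio and hands itself to a ConstantRotationComponent as owner.
; When PickupBehavior fires its player pickup event, it heals the VRPawn's character component by ContainedHealth and destroys itself.
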(event `self.ReceiveBeginPlay`
  (`/Game/blueprints/CustomComponents/RuneAnimationComponent.SetOwner` (`self.ConstantRotationComponent`) self)
  (`AudioComponent.Play` (`self.Audio`) 0.0))

(event `self.PickupBehavior.OnPlayerPickup`
  (params (PlayerRef :type "Actor Object Reference"))
  (bind _asvrpawn (cast `/Game/VRTemplate/Blueprints/VRPawn` PlayerRef))
  (`VRCharacterComponent.HealPlayer` (`/Game/VRTemplate/Blueprints/VRPawn.VRCharacterComp` _asvrpawn) (`self.ContainedHealth`))
  (`self.K2_DestroyActor`))

(fn `UserConstructionScript`)